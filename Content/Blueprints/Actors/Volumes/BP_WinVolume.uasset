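; BP_WinVolume is a level-exit volume that completes the level when the player overlaps it and no BP_Crystal actors remain.
; It checks for remaining crystals with a GetAllActorsOfClass query at overlap time.
; On completion, it finds the current level in the ordered LevelNames array and opens the next by name, wrapping to the first after the final level.
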(event Collision|EventActorBeginOverlap
  (params (OtherActor :type Actor%20Object%20Reference))
  (Utilities|IsPlayer OtherActor
    (:IsPlayer
      (if (not (CrystalManagement|AnyCrystalsRemaining))
        (LevelManagement|CompleteLevel)))))

(fn ConstructionScript)

(fn AnyCrystalsRemaining
  (bind _outactors (Actor|GetAllActorsOfClass "/Game/Blueprints/Actors/Collectables/BP_Crystal.BP_Crystal_C"))
  (return (> (Utilities|Array|Length _outactors) 0)))

(fn CompleteLevel
  (if (LevelManagement|IsFinalLevel)
    (LevelManagement|OpenFirstLevel)
    (else
      (LevelManagement|LoadNextLevel))))

(fn GetCurrentLevelIndex
  (bind _returnvalue (Game|GetCurrentLevelName true))
  (return (Utilities|Array|FindItem (Variables|Default|GetLevelNames) (Utilities|String|StringToName _returnvalue))))

(fn IsFinalLevel
  (return (== (Utilities|Array|LastIndex (Variables|Default|GetLevelNames)) (LevelManagement|GetCurrentLevelIndex))))

(fn LoadNextLevel
  (Game|OpenLevel(byName) (LevelManagement|GetNextLevelName)))

(fn GetNextLevelName
  (return (Utilities|Array|Get(acopy) (Variables|Default|GetLevelNames) (+ (LevelManagement|GetCurrentLevelIndex) 1))))

(fn OpenFirstLevel
  (Game|OpenLevel(byName) (Utilities|Array|Get(acopy) (Variables|Default|GetLevelNames))))