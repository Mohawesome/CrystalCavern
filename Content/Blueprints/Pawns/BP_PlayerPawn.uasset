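; Player pawn that rolls a physics sphere mesh and restarts the current level when it takes any damage.
; Forward/backward input applies torque to the sphere's X and Y axes as an acceleration change, while right/left input is unimplemented.
; The camera fades from opaque on BeginPlay.
; A once-only RestartLevel graph fades it back out, waits briefly, then reopens the level by name.
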(event EventBeginPlay
  (CameraFades|StartCameraFade :self (Game|GetPlayerCameraManager 0) :FromAlpha 1.0 :Duration 2.0 :bHoldWhenFinished true))

(event Game|Damage|EventAnyDamage
  (params (Damage :type Float%20%28single-precision%29) (DamageType :type Damage%20Type%20Object%20Reference) (InstigatedBy :type Controller%20Object%20Reference) (DamageCauser :type Actor%20Object%20Reference))
  (Utilities|RestartLevel))

(event Input|AxisEvents|InputAxisMoveForward/Backward
  (params (AxisValue :type Float%20%28single-precision%29))
  (bind _torquemultiplier (Variables|Default|GetTorqueMultiplier))
  (Class|PrimitiveComponent|AddTorqueinRadians (Variables|Default|GetSphere%20Static%20Mesh) (Math|Vector|MakeVector (* _torquemultiplier (stale Input|AxisEvents|InputAxisMoveRight/Left AxisValue)) (* AxisValue _torquemultiplier) 0.0) "None" true))

(event Input|AxisEvents|InputAxisMoveRight/Left
  (params (AxisValue :type Float%20%28single-precision%29)))

(fn ConstructionScript)