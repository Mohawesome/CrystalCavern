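; BP_Cannon is a cannon actor that automatically and repeatedly fires BP_Projectile once play begins.
; Each cycle waits for FireRate, spawns a scaled projectile at ProjectileSpawnPoint's world transform, then plays CannonFireTimeline to animate the barrel along its local Y axis.
; The timeline's Cannon Fired event track loops back to the delay, so the animation itself drives the next shot.
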(event EventBeginPlay
  (bind _projectile_spawn_point (Variables|Default|GetProjectile%20Spawn%20Point))
  (Utilities|FlowControl|Delay (Variables|CannonProperties|GetFireRate) :!label _label)
  (Game|SpawnActorfromClass "/Game/Blueprints/Actors/Projectiles/BP_Projectile.BP_Projectile_C" (Math|Transform|MakeTransform (Transformation|GetWorldLocation _projectile_spawn_point) (Transformation|GetWorldRotation _projectile_spawn_point) (Math|Conversions|ToVector(Float) (Variables|CannonProperties|GetProjectileScale))) "Undefined" 0 0)
  (bind _cannonbarrellocation (Timeline|Cannon%20Fire%20Timeline PlayFromStart)
    (:Update
      (Transformation|SetRelativeLocation (Variables|Default|GetCannonBarrel) (Math|Vector|MakeVector 0.0 _cannonbarrellocation 0.0) false false))
    (:CannonFired
      (goto _label))))

(fn ConstructionScript)